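; Multiplayer arena character Blueprint that handles player input for item handling and aim direction.
; Interact and Drop presses call client-named functions to collect or drop an item.
; CursorRight and CursorUp axes share one path that builds a planar vector and, past a deadzone, sets control rotation from it.
; A note marks this aiming logic for a move to C++, favoring a virtual cursor.
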(event Collision|EventActorBeginOverlap
  (params (OtherActor :type Actor%20Object%20Reference)))

(event Input|ActionEvents|InputActionInteract
  (params (Key :type Key%20Structure))
  (:Pressed
    (Class|TSArenaCharacterMP|ClientCollectItem)))

(event Input|ActionEvents|InputActionDrop
  (params (Key :type Key%20Structure))
  (:Pressed
    (Class|TSArenaCharacterMP|ClientDropItem)))

(event Input|AxisEvents|InputAxisCursorRight
  (params (AxisValue :type Float%20%28single-precision%29))
  ;[1 1 1] Move to C++ -> Virtual cursor would still be way better
  (if (>= (Math|Vector|VectorLength (Math|Vector|MakeVector (* (stale Input|AxisEvents|InputAxisCursorUp AxisValue) -1.0) AxisValue 0.0)) 0.4)
    (Pawn|SetControlRotation (Pawn|GetController) (Math|Conversions|RotationFromXVector (Math|Vector|MakeVector (* (stale Input|AxisEvents|InputAxisCursorUp AxisValue) -1.0) AxisValue 0.0)))))

(event Input|AxisEvents|InputAxisCursorUp
  (params (AxisValue :type Float%20%28single-precision%29))
  ;[1 1 1] Move to C++ -> Virtual cursor would still be way better
  (if (>= (Math|Vector|VectorLength (Math|Vector|MakeVector (* AxisValue -1.0) (stale Input|AxisEvents|InputAxisCursorRight AxisValue) 0.0)) 0.4)
    (Pawn|SetControlRotation (Pawn|GetController) (Math|Conversions|RotationFromXVector (Math|Vector|MakeVector (* AxisValue -1.0) (stale Input|AxisEvents|InputAxisCursorRight AxisValue) 0.0)))))

(fn ConstructionScript)